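; BP_Door_Static is a non-interactive, configurable door prop with no active runtime logic in its event graph.
; Its construction script scales the door mesh to the set width and height, relative to hard-coded base dimensions.
; It positions the separate handle mesh from the width, an offset and a handle height, so the handle is not stretched.
; A Flip option mirrors the assembly through negative Y scale on the root.
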(event EventBeginPlay)

(event Collision|EventActorBeginOverlap
  (params (OtherActor :type Actor%20Object%20Reference)))

(event EventTick
  (params (DeltaSeconds :type Float%20%28single-precision%29)))

(fn ConstructionScript
  (Transformation|SetRelativeScale3D (Variables|Default|GetSM_Door) (Math|Vector|MakeVector (/ (Variables|Default|GetDoor%20Width) 92.0) 1.0 (/ (Variables|Default|GetDoor%20Height) 236.0)))
  (Transformation|SetRelativeLocation (Variables|Default|GetSM_Handle) (Math|Vector|MakeVector (- (Variables|Default|GetDoor%20Width) (Variables|Default|GetHandle%20Offset)) (.y (Variables|/Script/Engine.SceneComponent|GetRelativeLocation (Variables|Default|GetSM_Door))) (Variables|Default|GetHandle%20Height)) false false)
  (Transformation|SetRelativeScale3D (Variables|Default|GetDefaultSceneRoot) (Math|Vector|MakeVector 1.0 (Math|Float|SelectFloat 1.0 -1.0 (Variables|Default|GetFlip)) 1.0)))