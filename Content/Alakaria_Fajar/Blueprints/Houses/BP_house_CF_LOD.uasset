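; Low-detail (LOD) house Blueprint for the CF facade type, with selectable facade variant, finish and mirroring.
; The construction script sets the facade mesh, mirrors it by negative Y scale, applies material and mobility, and writes a variant label to a text render.
; It also creates a dynamic window material for WindowsParallax, whose emissive brightness SetHousesLights switches between day and night values.
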(event EventSetHousesLights
  (params (On :type Boolean))
  (Rendering|Material|SetScalarParameterValue (Variables|Default|Getmat_dynamic_windows) "OverallEmissive" (Math|Float|SelectFloat (Variables|Default|GetWindow%20Brightness%20Night) (Variables|Default|GetWindow%20Brightness%20Day) On) :!class /Script/Engine.MaterialInstanceDynamic))

(fn ConstructionScript
  (|CallParentFunction)
  (Components|StaticMesh|SetStaticMesh (Variables|Default|Getsm_fasade) (Utilities|Select :Index (Variables|Default|GetFasade) :NewEnumerator0 "/Game/Alakaria_Fajar/Geometries/Houses_nanites/SM_CF1_LOD.SM_CF1_LOD" :NewEnumerator1 "/Game/Alakaria_Fajar/Geometries/Houses_nanites/SM_CF2_LOD.SM_CF2_LOD"))
  (Transformation|SetRelativeScale3D (Variables|Default|Getsm_fasade) (Math|Vector|MakeVector 1.0 (select (Variables|Default|GetMirrored) -1.0 1.0) 1.0))
  (Rendering|Components|TextRender|SetText (Variables|Default|GetTextRender) (Utilities|Text|ToText(String) (Utilities|String|Append "CF" "" (Utilities|String|EnumtoString (Variables|Default|GetFasade)) (Utilities|String|EnumtoString (Variables|Default|GetFinish)))))
  (Transformation|SetMobility (Variables|Default|Getsm_fasade) (Variables|Default|GetMobility))
  (Rendering|Material|SetMaterial (Variables|Default|Getsm_fasade) 0 (Utilities|Select :Index (Variables|Default|GetFinish) :NewEnumerator0 "/Game/Alakaria_Fajar/Materials/Exteriors/MI_WAT_exterior_fasadeA_New.MI_WAT_exterior_fasadeA_New" :NewEnumerator1 "/Game/Alakaria_Fajar/Materials/Exteriors/MI_WAT_exterior_fasadeA_New.MI_WAT_exterior_fasadeA_New"))
  (bind _returnvalue (Rendering|Material|CreateDynamicMaterialInstance "/Game/Alakaria_Fajar/Materials/Master/base_windowsrandom_Inst.base_windowsrandom_Inst" "None" "None" :!class /Script/Engine.KismetMaterialLibrary))
  (bind _output_get (Variables|Default|Setmat_dynamic_windows _returnvalue))
  (Rendering|Material|SetMaterial (Variables|Default|Getwindows_parallax) 0 _output_get))