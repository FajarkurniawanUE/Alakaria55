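; Base Blueprint for a villa that the player can look at and interact with to toggle its house info message.
; On BeginPlay it either passes HouseType to a floating marker widget placed above the actor's bounds or hides that widget, depending on MarkerUnit.
; Looking at its Box enables input and shows an interact hint with the villa type.
; Paired DoOnce gates make look-at and look-away each fire once, the latter disabling input and hiding the hint.
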(event EventBeginPlay
  (bind (_origin _boxextent) (Collision|GetActorBounds false false))
  (bind _widget (Variables|Default|GetWidget))
  (if (Variables|Default|GetMarker%20Unit)
    (bind _asumg_marker_unit (Utilities|Casting|CastToumg_marker_unit (UserInterface|GetUserWidgetObject _widget)))
    (Variables|/Game/Alakaria_Fajar/Blueprints/UMG/umg_marker_unit.umg_marker_unit_C|SetHouse%20Type _asumg_marker_unit (Variables|Default|GetHouse%20Type))
    (Transformation|SetWorldLocation (Variables|Default|GetWidget) (+ _origin (* (Transformation|GetActorUpVector) (.z _boxextent))) false false)
    (else
      (Rendering|SetVisibility _widget false false))))

(event EventOnLookedat
  (params (Player%20Character :type Actor%20Component%20Object%20Reference))
  (if (== Player%20Character (Variables|Default|GetBox))
    (Utilities|FlowControl|DoOnce false :!label _label
      (:Completed
        (Utilities|FlowControl|Sequence
          (:then_0
            (Input|EnableInput (Game|GetPlayerController 0))
            (Class|BPIUmg|ShowInteract(Message) (Game|GetPlayerController 0) true (Utilities|Text|ToText(String) (Utilities|String|Append "Villa " (Utilities|String|ToString(Text) (|GenerictoText (Variables|Default|GetHouse%20Type)))))))
          (:then_1
            (goto _label_2 Reset)))))
    (else
      (Utilities|FlowControl|DoOnce false :!label _label_2
        (:Completed
          (Utilities|FlowControl|Sequence
            (:then_0
              (goto _label Reset))
            (:then_1
              (Input|DisableInput (Game|GetPlayerController 0))
              (Class|BPIUmg|ShowInteract(Message) (Game|GetPlayerController 0) false))))))))

(event EventOnLookedAway
  (Utilities|FlowControl|DoOnce false
    (:Completed
      (Utilities|FlowControl|Sequence
        (:then_0
          (Utilities|FlowControl|DoOnce false) ; enters at Reset
        )
        (:then_1
          (Input|DisableInput (Game|GetPlayerController 0))
          (Class|BPIUmg|ShowInteract(Message) (Game|GetPlayerController 0) false))))))

(event Input|ActionEvents|InputActionInteract
  (params (Key :type Key%20Structure :default "None"))
  (:Released
    (Class|BPIUmg|ShowHouseInfo(Message) (Game|GetPlayerController 0) false (Variables|Default|GetHouse%20Type) true)))

(fn ConstructionScript)

(fn GetExteriorMode
  (return "NewEnumerator0"))

(fn GetIsGamepadKey
  (return false))