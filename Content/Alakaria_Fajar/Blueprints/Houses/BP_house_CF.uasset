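; BP_house_CF is a configurable CF-type house actor with switchable day and night lighting.
; Its construction script picks the facade mesh, finish material, mirroring and mobility, shows variant-specific components and labels the house.
; A dynamic material instance drives the parallax windows.
; Events toggle yard and facade lights while swapping window emissive level and curtain texture, or set window brightness directly.
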(event EventBeginPlay)

(event Collision|EventActorBeginOverlap
  (params (OtherActor :type Actor%20Object%20Reference)))

(event EventTick
  (params (DeltaSeconds :type Float%20%28single-precision%29)))

(event EventSetWindowsBrightness
  (params (Brightness :type Float%20%28double-precision%29))
  (bind _output_get (Variables|Default|SetWindows%20Brightness Brightness))
  (Rendering|Material|SetScalarParameterValue (Variables|Default|Getmat_dynamic_windows) "OverallEmissive" _output_get :!class /Script/Engine.MaterialInstanceDynamic))

(event EventSetHousesLights
  (params (On :type Boolean))
  (Rendering|SetVisibility (Variables|Default|Getcomp_light_yard1) On false)
  (Rendering|Material|SetScalarParameterValue (Variables|Default|Getmat_dynamic_windows) "OverallEmissive" (Math|Float|SelectFloat (Variables|Default|GetWindow%20Brightness%20Night) (Variables|Default|GetWindow%20Brightness%20Day) On) :!class /Script/Engine.MaterialInstanceDynamic)
  (Rendering|Material|SetTextureParameterValue (Variables|Default|Getmat_dynamic_windows) "Curtain" (select On "/Game/Alakaria_Fajar/Textures/T_Window_daytime.T_Window_daytime" "/Game/Alakaria_Fajar/Textures/T_Window_Curtains.T_Window_Curtains")))

(fn ConstructionScript
  (|CallParentFunction)
  (Components|StaticMesh|SetStaticMesh (Variables|Default|Getsm_fasade) (Utilities|Select :Index (Variables|Default|GetFasade) :NewEnumerator0 "/Game/Alakaria_Fajar/Geometries/Houses/SM_CF1_optimized.SM_CF1_optimized" :NewEnumerator1 "/Game/Alakaria_Fajar/Geometries/Houses/SM_CF2_optimized.SM_CF2_optimized"))
  (Transformation|SetRelativeScale3D (Variables|Default|Getsm_fasade) (Math|Vector|MakeVector 1.0 (select (Variables|Default|GetMirrored) -1.0 1.0) 1.0))
  (Rendering|Components|TextRender|SetText (Variables|Default|GetTextRender) (Utilities|Text|ToText(String) (Utilities|String|Append "CF" "" (Utilities|String|EnumtoString (Variables|Default|GetFasade)) (Utilities|String|EnumtoString (Variables|Default|GetFinish)))))
  (Transformation|SetMobility (Variables|Default|Getsm_fasade) (Variables|Default|GetMobility))
  (Rendering|Material|SetMaterial (Variables|Default|Getsm_fasade) 0 (Utilities|Select :Index (Variables|Default|GetFinish) :NewEnumerator0 "/Game/Alakaria_Fajar/Materials/Exteriors/MI_WAT_exterior_fasadeA_New2.MI_WAT_exterior_fasadeA_New2" :NewEnumerator1 "/Game/Alakaria_Fajar/Materials/Exteriors/MI_WAT_exterior_fasadeA_New2.MI_WAT_exterior_fasadeA_New2"))
  (bind _returnvalue (Rendering|Material|CreateDynamicMaterialInstance "/Game/Alakaria_Fajar/Materials/Master/base_windowsrandom_Inst.base_windowsrandom_Inst" "None" "None" :!class /Script/Engine.KismetMaterialLibrary))
  (bind _output_get (Variables|Default|Setmat_dynamic_windows _returnvalue))
  (Rendering|Material|SetMaterial (Variables|Default|Getwindows_parallax) 0 _output_get)
  (Variables|Default|SetHouse%20Type "NewEnumerator4")
  (Rendering|SetVisibility (Variables|Default|GetCube2_FS1) (Utilities|Select :Index (Variables|Default|GetFasade) :NewEnumerator0 true :NewEnumerator1 false) true)
  (Rendering|SetVisibility (Variables|Default|GetCube_FS2) (Utilities|Select :Index (Variables|Default|GetFasade) :NewEnumerator0 false :NewEnumerator1 true) true))