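; BP_Book_Stack procedurally builds a row of books along X as mesh instances in its construction script.
; When Refresh is off, it clears the instances and applies a dynamic material chosen by Type (General or Uniform) with texture, color and text settings.
; Randomize fills per-book size, depth, rotation and lean arrays from a seeded stream.
; Generation places the instances, using trigonometry to space leaning books.
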(fn ConstructionScript
  (if (not (Variables|Generation|GetRefresh))
    (Components|InstancedStaticMesh|ClearInstances (Variables|Default|GetInstancedBooks))
    (switch Utilities|FlowControl|Switch|Switchonenum_books (Variables|Generation|GetType)
      (:NewEnumerator0
        (Utilities|FlowControl|Sequence
          (:then_0
            (CallFunction|SetTexture (Variables|Generation|GetBook%20Texture) "/Game/Alakaria_Fajar/Blueprints/BookGen/Materials/Books/M_Book_Color1.M_Book_Color1"))
          (:then_1
            (CallFunction|Randomize))
          (:then_2
            (CallFunction|Generation))))
      (:NewEnumerator1
        (Utilities|FlowControl|Sequence
          (:then_0
            (CallFunction|SetTexture (Variables|Generation|GetBook%20Texture) "/Game/Alakaria_Fajar/Blueprints/BookGen/Materials/Books/M_Book_Uniform.M_Book_Uniform"))
          (:then_1
            (CallFunction|Randomize))
          (:then_2
            (CallFunction|Generation)))))))

(fn Generation
  (bind _bookmeshes (Variables|Generation|GetBookMeshes))
  (bind _lean (Variables|Randomize|GetLean))
  (bind _returnvalue (StaticMesh|GetBoundingBox _bookmeshes))
  (bind (_min _max) (Utilities|Struct|BreakBox _returnvalue))
  (bind _returnvalue_2 (- _max _min))
  (bind (_x _y _z) (Math|Vector|BreakVector _returnvalue_2))
  (for _index (range 0 (- (Variables|Generation|GetBookCount) 1))
    (bind _output_get (Variables|Default|SetCurrentXPosition (+ (Variables|Default|GetCurrentXPosition) (select (Utilities|Array|Get(acopy) (Variables|Default|GetLeanArray) _index) (+ (* (Math|Trig|Cos(Degrees) _lean) (* _x (* (Utilities|Array|Get(acopy) (Variables|Default|GetThicknessArray) _index) (.x (Variables|Generation|GetBook%20Scale))))) (* (Math|Trig|Sin(Degrees) _lean) (* (* _z (Utilities|Array|Get(acopy) (Variables|Default|GetHeightArray) _index)) (.z (Variables|Generation|GetBook%20Scale))))) (* _x (* (Utilities|Array|Get(acopy) (Variables|Default|GetThicknessArray) _index) (.x (Variables|Generation|GetBook%20Scale))))))))
    (Components|InstancedStaticMesh|AddInstance (Variables|Default|GetInstancedBooks) (Math|Transform|MakeTransform (Math|Vector|MakeVector (- _output_get (* _x (* (Utilities|Array|Get(acopy) (Variables|Default|GetThicknessArray) _index) (.x (Variables|Generation|GetBook%20Scale))))) (Utilities|Array|Get(acopy) (Variables|Default|GetDepthArray) _index) (Utilities|Array|Get(acopy) (Variables|Default|GetRotationArray) _index)) (Math|Rotator|MakeRotator (* (Utilities|Array|Get(acopy) (Variables|Default|GetRotationArray) _index) (Variables|Randomize|GetRotation)) (Math|Float|SelectFloat (Variables|Randomize|GetLean) 0.0 (Utilities|Array|Get(acopy) (Variables|Default|GetLeanArray) _index)) 0.0) (Math|Vector|MakeVector (* (Utilities|Array|Get(acopy) (Variables|Default|GetThicknessArray) _index) (.x (Variables|Generation|GetBook%20Scale))) (* (Utilities|Array|Get(acopy) (Variables|Default|GetWidthArray) _index) (.y (Variables|Generation|GetBook%20Scale))) (* (Utilities|Array|Get(acopy) (Variables|Default|GetHeightArray) _index) (.z (Variables|Generation|GetBook%20Scale))))) false)))

(fn Randomize
  (bind _rotation (Variables|Randomize|GetRotation))
  (bind _stream (Variables|Randomize|GetStream))
  (bind _height (Variables|Randomize|GetHeight))
  (bind _thickness (Variables|Randomize|GetThickness))
  (bind _width (Variables|Randomize|GetWidth))
  (bind _depth (Variables|Randomize|GetDepth))
  (bind _returnvalue (/ _rotation 1e+02))
  (bind _returnvalue_2 (Class|KismetMathLibrary|RandomBoolwithWeightfromStream _stream 0.1))
  (bind _returnvalue_3 (/ _height 1e+02))
  (bind _returnvalue_4 (/ _thickness 1e+02))
  (bind _returnvalue_5 (/ _width 1e+02))
  (bind _returnvalue_6 (/ _depth 1e+02))
  (for _index (range 0 (- (Variables|Generation|GetBookCount) 1))
    (Utilities|Array|SetArrayElem (Variables|Default|GetThicknessArray) _index (Math|Random|RandomFloatinRangefromStream (Variables|Randomize|GetStream) (- 1.0 _returnvalue_4) (+ _returnvalue_4 1.0)) true)
    (Utilities|Array|SetArrayElem (Variables|Default|GetHeightArray) _index (Math|Random|RandomFloatinRangefromStream (Variables|Randomize|GetStream) (- 1.0 _returnvalue_3) (+ _returnvalue_3 1.0)) true)
    (Utilities|Array|SetArrayElem (Variables|Default|GetWidthArray) _index (Math|Random|RandomFloatinRangefromStream (Variables|Randomize|GetStream) (- 1.0 _returnvalue_5) (+ _returnvalue_5 1.0)) true)
    (Utilities|Array|SetArrayElem (Variables|Default|GetDepthArray) _index (Math|Random|RandomFloatinRangefromStream (Variables|Randomize|GetStream) (- 1.0 _returnvalue_6) (+ _returnvalue_6 1.0)) true)
    (Utilities|Array|SetArrayElem (Variables|Default|GetRotationArray) _index (Math|Random|RandomFloatinRangefromStream (Variables|Randomize|GetStream) (- 1.0 _returnvalue) (+ _returnvalue 1.0)) true)
    (Utilities|Array|SetArrayElem (Variables|Default|GetLeanArray) _index (select (Math|Boolean|Equal(Boolean) _returnvalue_2 (Utilities|Array|Get(acopy) (Variables|Default|GetLeanArray) (- _index 1))) (Class|KismetSystemLibrary|MakeLiteralBool false) _returnvalue_2) true)))

(fn SetTexture
  (params (Book%20Texture :type Texture%20Object%20Reference) (Book%20Material :type Material%20Interface%20Object%20Reference))
  (Variables|Generation|SetBook%20Texture Book%20Texture)
  (Components|StaticMesh|SetStaticMesh (Variables|Default|GetInstancedBooks) (Variables|Generation|GetBookMeshes))
  (bind _returnvalue (Rendering|Material|CreateDynamicMaterialInstance Book%20Material "None" "None" :!class /Script/Engine.KismetMaterialLibrary))
  (Rendering|Material|SetTextureParameterValue _returnvalue "Texture4x4" (Variables|Generation|GetBook%20Texture))
  (Rendering|Material|SetVectorParameterValue _returnvalue "Base Color" (Variables|Uniform|GetColor%20Base) :!class /Script/Engine.MaterialInstanceDynamic)
  (Rendering|Material|SetVectorParameterValue _returnvalue "Text Color" (Variables|Uniform|GetColor%20Text) :!class /Script/Engine.MaterialInstanceDynamic)
  (Rendering|Material|SetScalarParameterValue _returnvalue "Text Roughness" (Variables|Uniform|GetText%20Roughness) :!class /Script/Engine.MaterialInstanceDynamic)
  (Rendering|Material|SetScalarParameterValue _returnvalue "Text Metalic" (Variables|Uniform|GetText%20Metalic) :!class /Script/Engine.MaterialInstanceDynamic)
  (Rendering|Material|SetMaterial (Variables|Default|GetInstancedBooks) 0 _returnvalue))