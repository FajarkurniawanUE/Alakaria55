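; Exterior planter Blueprint that holds an optional maple tree, its PLeaves component and two planter lights.
; The construction script gives the maple a random yaw and a slight random scale variation, and shows or hides tree and leaves through ShowTree.
; The PlantLightsOn event sets the visibility of both lights from its parameter.
; TreeSize and TreeRotation variables are unused.
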(event Custom|PlantLightsOn
  (params (bNewVisibility :type Boolean))
  (Rendering|SetVisibility (Variables|Default|Getcomp_light_planter) bNewVisibility false))

(event EventBeginPlay)

(event Collision|EventActorBeginOverlap
  (params (OtherActor :type Actor%20Object%20Reference)))

(event EventTick
  (params (DeltaSeconds :type Float%20%28single-precision%29)))

(fn ConstructionScript
  (Transformation|SetRelativeTransform (Variables|Default|GetSM_Maple08) (Math|Transform|MakeTransform "0, 0, 0" (Math|Rotator|MakeRotator 0.0 0.0 (Math|Random|RandomFloatinRange 0.0 3.6e+02)) (Math|Conversions|ToVector(Float) (Math|Random|RandomFloatinRange 0.5 0.6))) false false)
  (Rendering|SetVisibility (Variables|Default|GetSM_Maple08) (Variables|Default|GetShowTree) false))