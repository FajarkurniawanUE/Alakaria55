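; Point-of-interest Blueprint for exterior scenes that displays its own information through a umg_POI widget held in its Widget component.
; On BeginPlay it casts and caches that widget, then copies in its name, icon, color, image and description variables, so the content is set on the Blueprint.
; A HidePOI_info event collapses the widget's info border.
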(event Custom|HidePOI_info
  (Widget|SetVisibility (Variables|/Game/Alakaria_Fajar/Blueprints/UMG/umg_POI.umg_POI_C|GetBorder_POI_info (stale EventBeginPlay _asumg_poi)) "Collapsed"))

(event EventBeginPlay
  (bind _asumg_poi (Utilities|Casting|CastToumg_POI (UserInterface|GetUserWidgetObject (Variables|Default|GetWidget))))
  (Variables|/Game/Alakaria_Fajar/Blueprints/UMG/umg_POI.umg_POI_C|SetPOI%20Name _asumg_poi (Variables|Default|GetPOI%20Name))
  (Variables|/Game/Alakaria_Fajar/Blueprints/UMG/umg_POI.umg_POI_C|SetPOI%20Icon _asumg_poi (Variables|Default|GetPOI%20Icon))
  (Variables|/Game/Alakaria_Fajar/Blueprints/UMG/umg_POI.umg_POI_C|SetPOI%20Color _asumg_poi (Variables|Default|GetPOI%20Color))
  (Variables|/Game/Alakaria_Fajar/Blueprints/UMG/umg_POI.umg_POI_C|SetPOI%20Image _asumg_poi (Variables|Default|GetPOI%20Image))
  (Variables|/Game/Alakaria_Fajar/Blueprints/UMG/umg_POI.umg_POI_C|SetPOI%20Desc _asumg_poi (Variables|Default|GetPOI%20Desc)))

(fn ConstructionScript)