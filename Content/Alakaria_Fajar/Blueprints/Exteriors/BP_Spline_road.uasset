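; Spline road actor that lays a chosen mesh along its spline as spline mesh components built in the Construction Script.
; With UniformLength on, it places fixed MeshLength segments by distance, clamping tangents to that length and leaving any leftover spline uncovered.
; Otherwise it stretches one segment between each pair of spline points at unit scale, using the point tangents.
; The event graph has no active logic.
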(event EventBeginPlay)

(event Collision|EventActorBeginOverlap
  (params (OtherActor :type Actor%20Object%20Reference)))

(event EventTick
  (params (DeltaSeconds :type Float%20%28single-precision%29)))

(fn ConstructionScript
  (bind _returnvalue (Math|Vector2D|MakeVector2D 1.0 1.0))
  (bind _spline (Variables|Default|GetSpline))
  (bind _spline_2 (Variables|Default|GetSpline))
  (bind _spline_3 (Variables|Default|GetSpline))
  (bind _spline_4 (Variables|Default|GetSpline))
  (bind _meshlength (Variables|Default|GetMeshLength))
  (bind _returnvalue_2 (Spline|GetSplineLength _spline_4))
  (bind _returnvalue_3 (/ _returnvalue_2 _meshlength))
  (bind _returnvalue_4 (Math|Float|Truncate _returnvalue_3))
  (if (Variables|Default|GetUniform%20Length)
    (if (> _returnvalue_4 0)
      (for _index (range 0 (- _returnvalue_4 1))
        (bind _returnvalue_5 (AddComponent|AddSplineMeshComponent false))
        (Components|StaticMesh|SetStaticMesh _returnvalue_5 (Variables|Default|GetNew%20Mesh))
        (SplineMesh|SetStartandEnd _returnvalue_5 (Spline|GetLocationatDistanceAlongSpline _spline_3 (* _index (Variables|Default|GetMeshLength)) "Local") (Math|Vector|ClampVectorSize (Spline|GetTangentatDistanceAlongSpline _spline_3 (* _index (Variables|Default|GetMeshLength)) "Local") 1.0 (Variables|Default|GetMeshLength)) (Spline|GetLocationatDistanceAlongSpline _spline_2 (* (+ _index 1) (Variables|Default|GetMeshLength)) "Local") (Math|Vector|ClampVectorSize (Spline|GetTangentatDistanceAlongSpline _spline_2 (* (+ _index 1) (Variables|Default|GetMeshLength)) "Local") 1.0 (Variables|Default|GetMeshLength)) true :!class /Script/Engine.SplineMeshComponent)
        (Transformation|AttachComponentToComponent _returnvalue_5 (Variables|Default|GetSpline) "None" "KeepRelative" "KeepRelative" "KeepRelative" true)))
    (else
      (for _index_2 (range 0 (- (Spline|GetNumberOfSplinePoints _spline) 2))
        (bind _returnvalue_6 (AddComponent|AddSplineMeshComponent false))
        (Components|StaticMesh|SetStaticMesh _returnvalue_6 (Variables|Default|GetNew%20Mesh))
        (Transformation|AttachComponentToComponent _returnvalue_6 (Variables|Default|GetSpline) "None" "KeepRelative" "KeepRelative" "KeepRelative" true)
        (SplineMesh|SetStartScale _returnvalue_6 _returnvalue true :!class /Script/Engine.SplineMeshComponent)
        (SplineMesh|SetEndScale _returnvalue_6 _returnvalue true :!class /Script/Engine.SplineMeshComponent)
        (SplineMesh|SetStartandEnd _returnvalue_6 (.Location (Spline|GetLocationandTangentatSplinePoint _spline _index_2 "Local")) (.Tangent (Spline|GetLocationandTangentatSplinePoint _spline _index_2 "Local")) (.Location (Spline|GetLocationandTangentatSplinePoint _spline (+ _index_2 1) "Local")) (.Tangent (Spline|GetLocationandTangentatSplinePoint _spline (+ _index_2 1) "Local")) true :!class /Script/Engine.SplineMeshComponent)))))