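; Streetlamp exterior Blueprint, named as an LOD variant, with a light component and glowing lamp material that switch on and off.
; The construction script sets initial light visibility from the Lights variable and assigns a dynamic emissive material instance to the lamp mesh.
; The lightsOn and lightsOff events toggle the light's visibility and the material's Emissive parameter together.
; Random-delay, flicker-style visibility logic remains in the event graph but is disconnected and never runs.
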(event Custom|lightsOn
  (Rendering|SetVisibility (Variables|Default|Getcomp_light_streetlamp_LOD) true false)
  (Rendering|Material|SetScalarParameterValue (Variables|Default|Getmat_dynamic_emissive) "Emissive" 2.0 :!class /Script/Engine.MaterialInstanceDynamic))

(event Custom|lightsOff
  (Rendering|SetVisibility (Variables|Default|Getcomp_light_streetlamp_LOD) false false)
  (Rendering|Material|SetScalarParameterValue (Variables|Default|Getmat_dynamic_emissive) "Emissive" 0.0 :!class /Script/Engine.MaterialInstanceDynamic))

(fn ConstructionScript
  (Rendering|SetVisibility (Variables|Default|Getcomp_light_streetlamp_LOD) (Variables|Default|GetLights) false)
  (bind _returnvalue (Rendering|Material|CreateDynamicMaterialInstance "/Game/Alakaria_Fajar/Materials/Exteriors/MI_solid_emissive_streetlight.MI_solid_emissive_streetlight" "None" "None" :!class /Script/Engine.KismetMaterialLibrary))
  (bind _output_get (Variables|Default|Setmat_dynamic_emissive _returnvalue))
  (Rendering|Material|SetMaterial (Variables|Default|GetSM_streetLamp1) 1 _output_get))