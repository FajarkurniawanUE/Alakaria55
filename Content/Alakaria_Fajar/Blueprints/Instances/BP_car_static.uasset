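; Static car prop Blueprint that draws car bodies and their glass as two instanced mesh components, with meshes set by variables.
; The construction script assigns both meshes and loops over car instances to copy local transforms onto the glass component.
; It clears the car instances before that loop and adds none back, so the loop copies nothing as written.
; The event graph holds only empty events and an unconnected copy of the glass logic.
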(event EventBeginPlay)

(event Collision|EventActorBeginOverlap
  (params (OtherActor :type Actor%20Object%20Reference)))

(event EventTick
  (params (DeltaSeconds :type Float%20%28single-precision%29)))

(fn ConstructionScript
  (Components|InstancedStaticMesh|ClearInstances (Variables|Default|GetInstancedCar))
  (Components|StaticMesh|SetStaticMesh (Variables|Default|GetInstancedCar) (Variables|Default|GetSM_car))
  (Components|StaticMesh|SetStaticMesh (Variables|Default|GetInstancedGlasses) (Variables|Default|GetSM_glasses))
  (for _index (range 0 (- (Components|InstancedStaticMesh|GetInstanceCount (Variables|Default|GetInstancedCar)) 1))
    (Components|InstancedStaticMesh|AddInstance (Variables|Default|GetInstancedGlasses) (.OutInstanceTransform (Components|InstancedStaticMesh|GetInstanceTransform (Variables|Default|GetInstancedCar) _index false)) false)))