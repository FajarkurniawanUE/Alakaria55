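; Car instance manager that fills every BP_car_garage in the level with randomly chosen parked cars as instanced static meshes.
; Its construction script clears and rebuilds the instances from a seeded stream, so layouts are repeatable.
; Each garage usually gets one centered car, occasionally two offset sideways, with some yaws flipped 180 degrees.
; Cars 1-3 get matching window instances; car 4 has none and only appears in pairs.
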(event EventBeginPlay)

(event Collision|EventActorBeginOverlap
  (params (OtherActor :type Actor%20Object%20Reference)))

(event EventTick
  (params (DeltaSeconds :type Float%20%28single-precision%29)))

(fn ConstructionScript
  (bind _offset (Variables|Default|GetOffset))
  (Math|Random|SetRandomStreamSeed (Variables|Default|GetStreamSeed) (Variables|Default|GetRandomSeed))
  (Components|InstancedStaticMesh|ClearInstances (Variables|Default|GetISM_Car1))
  (Components|StaticMesh|SetStaticMesh (Variables|Default|GetISM_Car1) (Variables|Default|GetSM_car1))
  (Components|StaticMesh|SetStaticMesh (Variables|Default|GetISM_Car2) (Variables|Default|GetSM_car2))
  (Components|StaticMesh|SetStaticMesh (Variables|Default|GetISM_Car3) (Variables|Default|GetSM_car3))
  (Components|StaticMesh|SetStaticMesh (Variables|Default|GetISM_Car4) (Variables|Default|GetSM_car4))
  (Components|StaticMesh|SetStaticMesh (Variables|Default|GetISM_Windows2) (Variables|Default|GetSM_windows2))
  (Components|StaticMesh|SetStaticMesh (Variables|Default|GetISM_Windows1) (Variables|Default|GetSM_windows1))
  (Components|StaticMesh|SetStaticMesh (Variables|Default|GetISM_Windows3) (Variables|Default|GetSM_windows3))
  (bind _outactors (Actor|GetAllActorsOfClass "/Game/Alakaria_Fajar/Blueprints/Instances/BP_car_garage.BP_car_garage_C"))
  (for _array_element _outactors
    (switch int (Math|Integer|SelectInt 0 1 (Class|KismetMathLibrary|RandomBoolwithWeightfromStream (Variables|Default|GetStreamSeed) 0.2))
      (:0
        (for _array_element_2 (Utilities|Array|MakeArray _offset (* _offset -1.0))
          (switch int (Math|Random|RandomIntegerinRangefromStream (Variables|Default|GetStreamSeed) 0 3)
            (:0
              (bind _output_get (Variables|Default|SetLastTransform1 (Math|Transform|MakeTransform (+ (* (Math|Vector|GetRightVector (Variables|/Script/Engine.Actor|GetRootComponent _array_element)) _array_element_2) (.location (Transformation|GetWorldTransform (Variables|/Script/Engine.Actor|GetRootComponent _array_element)))) (Math|Rotator|MakeRotator (.Roll (Math|Rotator|BreakRotator (.rotation (Transformation|GetWorldTransform (Variables|/Script/Engine.Actor|GetRootComponent _array_element))))) (.Pitch (Math|Rotator|BreakRotator (.rotation (Transformation|GetWorldTransform (Variables|/Script/Engine.Actor|GetRootComponent _array_element))))) (Math|Float|SelectFloat (.Yaw (Math|Rotator|BreakRotator (.rotation (Transformation|GetWorldTransform (Variables|/Script/Engine.Actor|GetRootComponent _array_element))))) (+ (.Yaw (Math|Rotator|BreakRotator (.rotation (Transformation|GetWorldTransform (Variables|/Script/Engine.Actor|GetRootComponent _array_element))))) 1.8e+02) (Class|KismetMathLibrary|RandomBoolwithWeightfromStream (Variables|Default|GetStreamSeed) 0.8))))))
              (Components|InstancedStaticMesh|AddInstance (Variables|Default|GetISM_Car1) _output_get true)
              (Components|InstancedStaticMesh|AddInstance (Variables|Default|GetISM_Windows1) (Variables|Default|GetLastTransform1) true))
            (:1
              (bind _output_get_2 (Variables|Default|SetLastTransform1 (Math|Transform|MakeTransform (+ (* (Math|Vector|GetRightVector (Variables|/Script/Engine.Actor|GetRootComponent _array_element)) _array_element_2) (.location (Transformation|GetWorldTransform (Variables|/Script/Engine.Actor|GetRootComponent _array_element)))) (Math|Rotator|MakeRotator (.Roll (Math|Rotator|BreakRotator (.rotation (Transformation|GetWorldTransform (Variables|/Script/Engine.Actor|GetRootComponent _array_element))))) (.Pitch (Math|Rotator|BreakRotator (.rotation (Transformation|GetWorldTransform (Variables|/Script/Engine.Actor|GetRootComponent _array_element))))) (Math|Float|SelectFloat (.Yaw (Math|Rotator|BreakRotator (.rotation (Transformation|GetWorldTransform (Variables|/Script/Engine.Actor|GetRootComponent _array_element))))) (+ (.Yaw (Math|Rotator|BreakRotator (.rotation (Transformation|GetWorldTransform (Variables|/Script/Engine.Actor|GetRootComponent _array_element))))) 1.8e+02) (Class|KismetMathLibrary|RandomBoolwithWeightfromStream (Variables|Default|GetStreamSeed) 0.8))))))
              (Components|InstancedStaticMesh|AddInstance (Variables|Default|GetISM_Car2) _output_get_2 true)
              (Components|InstancedStaticMesh|AddInstance (Variables|Default|GetISM_Windows2) (Variables|Default|GetLastTransform1) true))
            (:2
              (bind _output_get_3 (Variables|Default|SetLastTransform1 (Math|Transform|MakeTransform (+ (* (Math|Vector|GetRightVector (Variables|/Script/Engine.Actor|GetRootComponent _array_element)) _array_element_2) (.location (Transformation|GetWorldTransform (Variables|/Script/Engine.Actor|GetRootComponent _array_element)))) (Math|Rotator|MakeRotator (.Roll (Math|Rotator|BreakRotator (.rotation (Transformation|GetWorldTransform (Variables|/Script/Engine.Actor|GetRootComponent _array_element))))) (.Pitch (Math|Rotator|BreakRotator (.rotation (Transformation|GetWorldTransform (Variables|/Script/Engine.Actor|GetRootComponent _array_element))))) (Math|Float|SelectFloat (.Yaw (Math|Rotator|BreakRotator (.rotation (Transformation|GetWorldTransform (Variables|/Script/Engine.Actor|GetRootComponent _array_element))))) (+ (.Yaw (Math|Rotator|BreakRotator (.rotation (Transformation|GetWorldTransform (Variables|/Script/Engine.Actor|GetRootComponent _array_element))))) 1.8e+02) (Class|KismetMathLibrary|RandomBoolwithWeightfromStream (Variables|Default|GetStreamSeed) 0.8))))))
              (Components|InstancedStaticMesh|AddInstance (Variables|Default|GetISM_Car3) _output_get_3 true)
              (Components|InstancedStaticMesh|AddInstance (Variables|Default|GetISM_Windows3) (Variables|Default|GetLastTransform1) true))
            (:3
              (Components|InstancedStaticMesh|AddInstance (Variables|Default|GetISM_Car4) (Math|Transform|MakeTransform (+ (* (Math|Vector|GetRightVector (Variables|/Script/Engine.Actor|GetRootComponent _array_element)) _array_element_2) (.location (Transformation|GetWorldTransform (Variables|/Script/Engine.Actor|GetRootComponent _array_element)))) (Math|Rotator|MakeRotator (.Roll (Math|Rotator|BreakRotator (.rotation (Transformation|GetWorldTransform (Variables|/Script/Engine.Actor|GetRootComponent _array_element))))) (.Pitch (Math|Rotator|BreakRotator (.rotation (Transformation|GetWorldTransform (Variables|/Script/Engine.Actor|GetRootComponent _array_element))))) (Math|Float|SelectFloat (.Yaw (Math|Rotator|BreakRotator (.rotation (Transformation|GetWorldTransform (Variables|/Script/Engine.Actor|GetRootComponent _array_element))))) (+ (.Yaw (Math|Rotator|BreakRotator (.rotation (Transformation|GetWorldTransform (Variables|/Script/Engine.Actor|GetRootComponent _array_element))))) 1.8e+02) (Class|KismetMathLibrary|RandomBoolwithWeightfromStream (Variables|Default|GetStreamSeed) 0.8)))) true)))))
      (:1
        (switch int (Math|Random|RandomIntegerinRangefromStream (Variables|Default|GetStreamSeed) 0 2)
          (:0
            (bind _output_get_4 (Variables|Default|SetLastTransform1 (Math|Transform|MakeTransform (.location (Transformation|GetWorldTransform (Variables|/Script/Engine.Actor|GetRootComponent _array_element))) (Math|Rotator|MakeRotator (.Roll (Math|Rotator|BreakRotator (.rotation (Transformation|GetWorldTransform (Variables|/Script/Engine.Actor|GetRootComponent _array_element))))) (.Pitch (Math|Rotator|BreakRotator (.rotation (Transformation|GetWorldTransform (Variables|/Script/Engine.Actor|GetRootComponent _array_element))))) (Math|Float|SelectFloat (.Yaw (Math|Rotator|BreakRotator (.rotation (Transformation|GetWorldTransform (Variables|/Script/Engine.Actor|GetRootComponent _array_element))))) (+ (.Yaw (Math|Rotator|BreakRotator (.rotation (Transformation|GetWorldTransform (Variables|/Script/Engine.Actor|GetRootComponent _array_element))))) 1.8e+02) (Class|KismetMathLibrary|RandomBoolwithWeightfromStream (Variables|Default|GetStreamSeed) 0.8))))))
            (Components|InstancedStaticMesh|AddInstance (Variables|Default|GetISM_Car1) _output_get_4 true)
            (Components|InstancedStaticMesh|AddInstance (Variables|Default|GetISM_Windows1) (Variables|Default|GetLastTransform1) true))
          (:1
            (bind _output_get_5 (Variables|Default|SetLastTransform1 (Math|Transform|MakeTransform (.location (Transformation|GetWorldTransform (Variables|/Script/Engine.Actor|GetRootComponent _array_element))) (Math|Rotator|MakeRotator (.Roll (Math|Rotator|BreakRotator (.rotation (Transformation|GetWorldTransform (Variables|/Script/Engine.Actor|GetRootComponent _array_element))))) (.Pitch (Math|Rotator|BreakRotator (.rotation (Transformation|GetWorldTransform (Variables|/Script/Engine.Actor|GetRootComponent _array_element))))) (Math|Float|SelectFloat (.Yaw (Math|Rotator|BreakRotator (.rotation (Transformation|GetWorldTransform (Variables|/Script/Engine.Actor|GetRootComponent _array_element))))) (+ (.Yaw (Math|Rotator|BreakRotator (.rotation (Transformation|GetWorldTransform (Variables|/Script/Engine.Actor|GetRootComponent _array_element))))) 1.8e+02) (Class|KismetMathLibrary|RandomBoolwithWeightfromStream (Variables|Default|GetStreamSeed) 0.8))))))
            (Components|InstancedStaticMesh|AddInstance (Variables|Default|GetISM_Car2) _output_get_5 true)
            (Components|InstancedStaticMesh|AddInstance (Variables|Default|GetISM_Windows2) (Variables|Default|GetLastTransform1) true))
          (:2
            (bind _output_get_6 (Variables|Default|SetLastTransform1 (Math|Transform|MakeTransform (.location (Transformation|GetWorldTransform (Variables|/Script/Engine.Actor|GetRootComponent _array_element))) (Math|Rotator|MakeRotator (.Roll (Math|Rotator|BreakRotator (.rotation (Transformation|GetWorldTransform (Variables|/Script/Engine.Actor|GetRootComponent _array_element))))) (.Pitch (Math|Rotator|BreakRotator (.rotation (Transformation|GetWorldTransform (Variables|/Script/Engine.Actor|GetRootComponent _array_element))))) (Math|Float|SelectFloat (.Yaw (Math|Rotator|BreakRotator (.rotation (Transformation|GetWorldTransform (Variables|/Script/Engine.Actor|GetRootComponent _array_element))))) (+ (.Yaw (Math|Rotator|BreakRotator (.rotation (Transformation|GetWorldTransform (Variables|/Script/Engine.Actor|GetRootComponent _array_element))))) 1.8e+02) (Class|KismetMathLibrary|RandomBoolwithWeightfromStream (Variables|Default|GetStreamSeed) 0.8))))))
            (Components|InstancedStaticMesh|AddInstance (Variables|Default|GetISM_Car3) _output_get_6 true)
            (Components|InstancedStaticMesh|AddInstance (Variables|Default|GetISM_Windows3) (Variables|Default|GetLastTransform1) true))
          (:3
            (Components|InstancedStaticMesh|AddInstance (Variables|Default|GetISM_Car4) (Math|Transform|MakeTransform (.location (Transformation|GetWorldTransform (Variables|/Script/Engine.Actor|GetRootComponent _array_element))) (Math|Rotator|MakeRotator (.Roll (Math|Rotator|BreakRotator (.rotation (Transformation|GetWorldTransform (Variables|/Script/Engine.Actor|GetRootComponent _array_element))))) (.Pitch (Math|Rotator|BreakRotator (.rotation (Transformation|GetWorldTransform (Variables|/Script/Engine.Actor|GetRootComponent _array_element))))) (Math|Float|SelectFloat (.Yaw (Math|Rotator|BreakRotator (.rotation (Transformation|GetWorldTransform (Variables|/Script/Engine.Actor|GetRootComponent _array_element))))) (+ (.Yaw (Math|Rotator|BreakRotator (.rotation (Transformation|GetWorldTransform (Variables|/Script/Engine.Actor|GetRootComponent _array_element))))) 1.8e+02) (Class|KismetMathLibrary|RandomBoolwithWeightfromStream (Variables|Default|GetStreamSeed) 0.8)))) true)))))))