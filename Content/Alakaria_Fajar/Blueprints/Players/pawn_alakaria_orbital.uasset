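; Orbital camera pawn for the Alakaria Fajar project, providing a look-around view restricted to downward angles.
; On possession it clamps the player camera manager's pitch range, and Turn and LookUp axes drive controller rotation scaled by look sensitivity and delta time.
; The MoveRight axis is forwarded to the player controller as a sun slider message.
; Calls for orbital play mode and initial mode messages are present but unconnected.
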(event EventBeginPlay)

(event Collision|EventActorBeginOverlap
  (params (OtherActor :type Actor%20Object%20Reference)))

(event EventTick
  (params (DeltaSeconds :type Float%20%28single-precision%29)))

(event EventPossessed
  (params (NewController :type Controller%20Object%20Reference))
  (bind _returnvalue (Game|GetPlayerCameraManager 0))
  (Utilities|FlowControl|Sequence
    (:then_0
      (Variables|/Script/Engine.PlayerCameraManager|SetViewPitchMin _returnvalue -9e+01)
      (Variables|/Script/Engine.PlayerCameraManager|SetViewPitchMax _returnvalue -25.0))))

(event Input|AxisEvents|InputAxisLookUp
  (params (AxisValue :type Float%20%28single-precision%29))
  ;[0.15 0.15 0.15 0.5] mouse gamepad look
  (Pawn|Input|AddControllerPitchInput (* (* AxisValue (Variables|Default|GetlookSensitivity)) (Utilities|Time|GetWorldDeltaSeconds))))

(event Input|AxisEvents|InputAxisTurn
  (params (AxisValue :type Float%20%28single-precision%29))
  ;[0.15 0.15 0.15 0.5] mouse gamepad look
  (Pawn|Input|AddControllerYawInput (* (* AxisValue (Variables|Default|GetlookSensitivity)) (Utilities|Time|GetWorldDeltaSeconds))))

(event Input|AxisEvents|InputAxisMoveRight
  (params (AxisValue :type Float%20%28single-precision%29))
  (Class|BPIUmg|MoveSunSlider(Message) (Game|GetPlayerController 0) AxisValue))

(fn ConstructionScript)