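; First-person walking character for Alakaria with mouse and gamepad look, sprint, and a CineCamera lens.
; Timelines lerp focal length for a toggled fisheye and hold-to-zoom; a looping timer traces ahead while zooming to set smoothed focus distance.
; A per-tick short trace sends looked-at and looked-away messages to BPI_umg actors, using a DoOnce to fire look-away once.
; In slider mode, MoveRight input also drives the player controller's sun slider.
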(event Custom|tracingInteraction
  (bind _camera (Variables|Default|GetCamera))
  (bind _returnvalue (Transformation|GetWorldLocation _camera))
  ;[0.15 0.15 0.15 0.5] line trace zoom
  (Utilities|IsValid (Game|GetPlayerCharacter 0)
    (:Is%20Valid
      (bind (_outhit _returnvalue_2) (Collision|LineTraceByChannel _returnvalue (+ _returnvalue (* (Math|Vector|GetForwardVector (.Rotation (Math|Transform|BreakTransform (Transformation|GetWorldTransform (Variables|Default|GetCineCamera))))) 5e+02)) "TraceTypeQuery1" false 0 "None"))
      (if _returnvalue_2
        (if (Utilities|DoesObjectImplementInterface (Components|GetOwner (.HitComponent (Collision|BreakHitResult _outhit))) "/Game/Alakaria_Fajar/Blueprints/UMG/BPI_umg.BPI_umg_C")
          (Utilities|FlowControl|Sequence
            (:then_0
              (Class|BPIUmg|OnLookedat(Message) (Components|GetOwner (.HitComponent (Collision|BreakHitResult _outhit))) (.HitComponent (Collision|BreakHitResult _outhit)))
              (Variables|Default|SetTracedActor (Components|GetOwner (.HitComponent (Collision|BreakHitResult _outhit)))))
            (:then_1
              (goto _label Reset)))
          (else
            (Utilities|FlowControl|DoOnce false :!label _label
              (:Completed
                (Class|BPIUmg|OnLookedAway(Message) (Variables|Default|GetTracedActor))
                (Variables|Default|SetTracedActor 0)))))
        (else
          (goto _label))))
    (:Is%20Not%20Valid
      (goto _label))))

(event Custom|StartTrace
  ;[0.15 0.15 0.15 0.5] line trace zoom
  (Utilities|Time|SetTimerbyEvent (delegate Custom|TracingZoom) 0.2 true))

(event Custom|TracingZoom
  (bind _camera (Variables|Default|GetCamera))
  (bind _returnvalue (Transformation|GetWorldLocation _camera))
  ;[0.15 0.15 0.15 0.5] line trace zoom
  (if (Variables|Default|GetisZooming)
    (bind (_outhit _returnvalue_2) (Collision|LineTraceByChannel _returnvalue (+ _returnvalue (* (Math|Vector|GetForwardVector (.Rotation (Math|Transform|BreakTransform (Transformation|GetWorldTransform (Variables|Default|GetCineCamera))))) 1.6e+03)) "TraceTypeQuery1" false 0 "None"))
    (Variables|/Script/CinematicCamera.CineCameraComponent|SetFocusSettings (Variables|Default|GetCineCamera) (Utilities|Struct|MakeCameraFocusSettings "Manual" (Math|Float|SelectFloat (.Distance (Collision|BreakHitResult _outhit)) 1e+09 _returnvalue_2) "(ActorToTrack=None,RelativeOffset=(X=0.000000,Y=0.000000,Z=0.000000))" true 2e+01))))

(event EventPossessed
  (params (NewController :type Controller%20Object%20Reference))
  (bind _returnvalue (Game|GetPlayerCameraManager 0))
  (Utilities|FlowControl|Sequence
    (:then_0
      (Variables|/Script/Engine.PlayerCameraManager|SetViewPitchMin _returnvalue -9e+01)
      (Variables|/Script/Engine.PlayerCameraManager|SetViewPitchMax _returnvalue 9e+01))
    (:then_1
      (CallFunction|StartTrace))))

(event EventTick
  (params (DeltaSeconds :type Float%20%28single-precision%29))
  ;[0.15 0.15 0.15 0.5] line trace zoom
  (CallFunction|TracingInteraction))

(event Input|ActionEvents|InputActionFisheye
  (params (Key :type Key%20Structure :default "None"))
  (:Released
    (Utilities|FlowControl|FlipFlop
      (:A
        (Variables|Default|SetIsFisheye true)
        (bind _newtrack_0 (Timeline|Timeline PlayFromStart)
          (:Update
            (Variables|/Script/CinematicCamera.CineCameraComponent|SetCurrentFocalLength (Variables|Default|GetCineCamera) (Math|Float|Lerp (Variables|Default|GetdefaultFOV) (Variables|Default|GetfisheyeFOV) _newtrack_0)))))
      (:B
        (Variables|Default|SetIsFisheye false)
        (Timeline|Timeline ReverseFromEnd)))))

(event Input|ActionEvents|InputActionSprint
  (params (Key :type Key%20Structure :default "None"))
  (bind _charactermovement (Variables|Character|GetCharacterMovement))
  ;[0.15 0.15 0.15 0.5] sprint
  (:Pressed
    (Variables|/Script/Engine.CharacterMovementComponent|SetMaxWalkSpeed _charactermovement (* (Variables|Default|GetspeedSprint) (Variables|Default|GetspeedMultiplier))))
  (:Released
    (Variables|/Script/Engine.CharacterMovementComponent|SetMaxWalkSpeed _charactermovement (* (Variables|Default|GetspeedWalk) (Variables|Default|GetspeedMultiplier)))))

(event Input|ActionEvents|InputActionZoom
  (params (Key :type Key%20Structure :default "None"))
  ;[0.15 0.15 0.15 0.5] Zoom
  (:Pressed
    (Variables|Default|SetisZooming true)
    (bind _newtrack_0 (Timeline|Timeline_zoom Play)
      (:Update
        (Variables|/Script/CinematicCamera.CineCameraComponent|SetCurrentFocalLength (Variables|Default|GetCineCamera) (Math|Float|Lerp (select (Variables|Default|GetIsFisheye) (Variables|Default|GetfisheyeFOV) (Variables|Default|GetdefaultFOV)) (Variables|Default|GetzoomFOV) _newtrack_0)))))
  (:Released
    (Variables|Default|SetisZooming false)
    (Variables|/Script/CinematicCamera.CineCameraComponent|SetFocusSettings (Variables|Default|GetCineCamera) (Utilities|Struct|MakeCameraFocusSettings "Disable" 1e+05 "(ActorToTrack=None,RelativeOffset=(X=0.000000,Y=0.000000,Z=0.000000))" true))
    (Timeline|Timeline_zoom Reverse)))

(event Input|AxisEvents|InputAxisMoveForward
  (params (AxisValue :type Float%20%28single-precision%29))
  (bind _returnvalue (Pawn|GetControlRotation :!class /Script/Engine.Pawn))
  (bind (_roll _pitch _yaw) (Math|Rotator|BreakRotator _returnvalue))
  ;[0.15 0.15 0.15 0.5] movement
  (Pawn|Input|AddMovementInput (Math|Vector|GetForwardVector (Math|Rotator|MakeRotator _roll 0.0 _yaw)) AxisValue false))

(event Input|AxisEvents|InputAxisTurnGamepad
  (params (AxisValue :type Float%20%28single-precision%29))
  (Pawn|Input|AddControllerYawInput (* AxisValue (Variables|Default|GetlookSensitivity))))

(event Input|AxisEvents|InputAxisLookUpGamepad
  (params (AxisValue :type Float%20%28single-precision%29))
  (Pawn|Input|AddControllerPitchInput (* AxisValue (Variables|Default|GetlookSensitivity))))

(event Input|AxisEvents|InputAxisMoveRight
  (params (AxisValue :type Float%20%28single-precision%29))
  (if (Variables|Default|GetSliderMode)
    (Class|BPIUmg|MoveSunSlider(Message) (Game|GetPlayerController 0) AxisValue)))

(event Input|AxisEvents|InputAxisMoveRight
  (params (AxisValue :type Float%20%28single-precision%29))
  (bind _returnvalue (Pawn|GetControlRotation :!class /Script/Engine.Pawn))
  (bind (_roll _pitch _yaw) (Math|Rotator|BreakRotator _returnvalue))
  ;[0.15 0.15 0.15 0.5] movement
  (Pawn|Input|AddMovementInput (Math|Vector|GetRightVector (Math|Rotator|MakeRotator _roll 0.0 _yaw)) AxisValue false))

(event Input|AxisEvents|InputAxisTurnMouse
  (params (AxisValue :type Float%20%28single-precision%29))
  ;[0.15 0.15 0.15 0.5] mouse gamepad look
  (Pawn|Input|AddControllerYawInput (* AxisValue (Variables|Default|GetlookMouseSensitivity) (Math|Float|SelectFloat -1.0 1.0 (Variables|Default|GetInvertLookMouse)))))

(event Input|AxisEvents|InputAxisLookUpMouse
  (params (AxisValue :type Float%20%28single-precision%29))
  ;[0.15 0.15 0.15 0.5] mouse gamepad look
  (Pawn|Input|AddControllerPitchInput (* AxisValue (Variables|Default|GetlookMouseSensitivity) (Math|Float|SelectFloat -1.0 1.0 (Variables|Default|GetInvertLookMouse)))))

(fn ConstructionScript)