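; Dollhouse view pawn for Alakaria that gives the player orbital-style look control.
; On possession it limits camera pitch to between straight down and level, then calls the player controller's orbital mode message.
; Mouse and gamepad axes drive controller yaw and pitch, scaled by look sensitivity and frame time.
; The gamepad invert option flips both axes, while mouse input has no inversion.
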(event EventPossessed
  (params (NewController :type Controller%20Object%20Reference))
  (bind _returnvalue (Game|GetPlayerCameraManager 0))
  (Utilities|FlowControl|Sequence
    (:then_0
      (Variables|/Script/Engine.PlayerCameraManager|SetViewPitchMin _returnvalue -9e+01)
      (Variables|/Script/Engine.PlayerCameraManager|SetViewPitchMax _returnvalue 0.0))
    (:then_1
      (Class|BPIUmg|PlayModeOrbital(Message) (Game|GetPlayerController 0)))))

(event Input|AxisEvents|InputAxisTurnMouse
  (params (AxisValue :type Float%20%28single-precision%29))
  ;[0.15 0.15 0.15 0.5] mouse gamepad look
  (Pawn|Input|AddControllerYawInput (* (* AxisValue (Variables|Default|GetlookSensitivity)) (Utilities|Time|GetWorldDeltaSeconds))))

(event Input|AxisEvents|InputAxisLookUpMouse
  (params (AxisValue :type Float%20%28single-precision%29))
  ;[0.15 0.15 0.15 0.5] mouse gamepad look
  (Pawn|Input|AddControllerPitchInput (* (* AxisValue (Variables|Default|GetlookSensitivity)) (Utilities|Time|GetWorldDeltaSeconds))))

(event Input|AxisEvents|InputAxisTurnGamepad
  (params (AxisValue :type Float%20%28single-precision%29))
  (Pawn|Input|AddControllerYawInput (* (* AxisValue (Variables|Default|GetlookSensitivity) (Math|Float|SelectFloat -1.0 1.0 (Variables|Default|GetInvertLookGamepad))) (Utilities|Time|GetWorldDeltaSeconds))))

(event Input|AxisEvents|InputAxisLookUpGamepad
  (params (AxisValue :type Float%20%28single-precision%29))
  (Pawn|Input|AddControllerPitchInput (* (* AxisValue (Variables|Default|GetlookSensitivity) (Math|Float|SelectFloat -1.0 1.0 (Variables|Default|GetInvertLookGamepad))) (Utilities|Time|GetWorldDeltaSeconds))))

(fn ConstructionScript)