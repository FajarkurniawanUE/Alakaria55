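; Player controller for the Alakaria exterior villa showcase, switching between a walk character and an orbital pawn with a camera blend and delayed possession.
; It owns the exterior HUD and tracks one active window (menu, teleport, guide, house info) to set input mode and movement.
; Orbital mode shows the sun slider and POI markers.
; It also fills house info from a data table, opens levels behind a loading screen and maps numpad DLSS switching.
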(event Custom|SetHouseInfo
  (params (House%20Type :type enum_house_type%20Enum :default "NewEnumerator0"))
  ;[0.15 0.15 0.15 0.5] house info
  (bind _outrownames (DataTable|GetDataTableRowNames "/Game/Alakaria_Fajar/Blueprints/Database/datatable_houses.datatable_houses"))
  (for _array_element _outrownames
    (bind _returnvalue (Utilities|GetDataTableRow "/Game/Alakaria_Fajar/Blueprints/Database/datatable_houses.datatable_houses" _array_element)
      (:then
        (if (== (.Type (Utilities|Struct|Breakstruct_houses _returnvalue)) (Math|Conversions|ToInteger(Byte) House%20Type))
          (Default|SetHouseInfo (Variables|/Game/Alakaria_Fajar/Blueprints/UMG/umg_exterior.umg_exterior_C|Getumg_house_info (Variables|Default|Getumg_exterior)) House%20Type (.NumofRooms (Utilities|Struct|Breakstruct_houses _returnvalue)) (.VillaArea (Utilities|Struct|Breakstruct_houses _returnvalue)) (.PlotArea (Utilities|Struct|Breakstruct_houses _returnvalue)) (.Gallery (Utilities|Struct|Breakstruct_houses _returnvalue)) (.Level (Utilities|Struct|Breakstruct_houses _returnvalue)) (.Description (Utilities|Struct|Breakstruct_houses _returnvalue)) (.ImageLoading (Utilities|Struct|Breakstruct_houses _returnvalue))))))))

(event Custom|TogglePOI
  (params (bNewVisibility :type Boolean))
  ;[0.15 0.15 0.15 0.5] point of interest
  (bind _outactors (Actor|GetAllActorsOfClass "/Game/Alakaria_Fajar/Blueprints/Exteriors/bp_POI.bp_POI_C"))
  (for _array_element _outactors
    (Rendering|SetVisibility (Variables|/Game/Alakaria_Fajar/Blueprints/Exteriors/bp_POI.bp_POI_C|GetWidget _array_element) bNewVisibility false)
    (Default|HidePOIInfo _array_element)))

(event EventBeginPlay
  ;[0.15 0.15 0.15 0.5] begin play
  (Utilities|FlowControl|Sequence
    (:then_0
      (bind _returnvalue (UserInterface|CreateWidget "/Game/Alakaria_Fajar/Blueprints/UMG/umg_exterior.umg_exterior_C"))
      (bind _output_get (Variables|Default|Setumg_exterior _returnvalue))
      (UserInterface|Viewport|AddtoViewport _output_get 0))
    (:then_1
      (bind _outactors (Actor|GetAllActorsOfClass "/Game/Alakaria_Fajar/Blueprints/Players/char_alakaria_walk.char_alakaria_walk_C"))
      (Utilities|IsValid (Utilities|Array|Get(acopy) _outactors)
        (:Is%20Valid
          (Variables|Default|Setchar_akaria_walk (Utilities|Array|Get(acopy) _outactors)))))
    (:then_2
      (bind _outactors_2 (Actor|GetAllActorsOfClass "/Game/Alakaria_Fajar/Blueprints/Players/pawn_alakaria_orbital.pawn_alakaria_orbital_C"))
      (Utilities|IsValid (Utilities|Array|Get(acopy) _outactors_2)
        (:Is%20Valid
          (Variables|Default|Setpawn_alakaria_orbital (Utilities|Array|Get(acopy) _outactors_2)))))
    (:then_3
      (bind _output_get_2 (Variables|Default|SetExterior%20Mode (Variables|Default|GetExterior%20Mode)))
      (switch Utilities|FlowControl|Switch|Switchonenum_exterior_mode _output_get_2
        (:NewEnumerator0
          (Pawn|Possess (Variables|Default|Getchar_akaria_walk)))
        (:NewEnumerator1
          (Pawn|Possess (Variables|Default|Getpawn_alakaria_orbital))))
      (CallFunction|ShowGuide true))))

(event EventSetIsGamepadKey
  (params (Gamepad :type Boolean))
  (Variables|Default|SetGamepadKey Gamepad))

(event EventShowSunSlider
  (params (Show :type Boolean))
  ;[0.15 0.15 0.15 0.5] sun slider
  (Default|ToggleSunslider (Variables|Default|Getumg_exterior) Show)
  (CallFunction|TogglePOI Show))

(event EventShowInteract
  (params (Show :type Boolean) (Hint :type Text))
  (bind _umg_exterior (Variables|Default|Getumg_exterior))
  ;[0.15 0.15 0.15 0.5] interact crosshair
  (Default|ToggleInteract _umg_exterior Show Hint)
  (Default|SetInteractButton (Variables|/Game/Alakaria_Fajar/Blueprints/UMG/umg_exterior.umg_exterior_C|Getumg_crosshair _umg_exterior) (Variables|Default|GetGamepadKey)))

(event EventLoadingOpenLevel
  (params (VillaType :type Text) (Desc :type Text) (Image%20Loading :type Texture%202D%20Object%20Reference) (Level%20Name :type Name :default "None"))
  ;[0.15 0.15 0.15 0.5] loading open level
  (bind _returnvalue (UserInterface|CreateWidget "/Game/Alakaria_Fajar/Blueprints/UMG/umg_loadingscreen.umg_loadingscreen_C"))
  (Variables|/Game/Alakaria_Fajar/Blueprints/UMG/umg_loadingscreen.umg_loadingscreen_C|Setname_unit _returnvalue VillaType)
  (Variables|/Game/Alakaria_Fajar/Blueprints/UMG/umg_loadingscreen.umg_loadingscreen_C|Setdesc_unit _returnvalue Desc)
  (Variables|/Game/Alakaria_Fajar/Blueprints/UMG/umg_loadingscreen.umg_loadingscreen_C|Setimg_unit_loading _returnvalue Image%20Loading)
  (UserInterface|Viewport|AddtoViewport _returnvalue 0)
  (Utilities|FlowControl|Delay 1.0)
  (Game|OpenLevel(byName) Level%20Name))

(event EventMoveSunSlider
  (params (Value :type Float%20%28double-precision%29))
  (bind _umg_exterior (Variables|Default|Getumg_exterior))
  (bind _umg_sunslider (Variables|/Game/Alakaria_Fajar/Blueprints/UMG/umg_exterior.umg_exterior_C|Getumg_sunslider _umg_exterior))
  (bind _slider_67 (Variables|/Game/Alakaria_Fajar/Blueprints/UMG/umg_sunslider.umg_sunslider_C|GetSlider_67 _umg_sunslider))
  (bind _returnvalue (Class|Slider|GetValue _slider_67))
  ;[0.15 0.15 0.15 0.5] sun slider
  (if (>= _returnvalue 1.0)
    (Class|Slider|SetValue (Variables|/Game/Alakaria_Fajar/Blueprints/UMG/umg_sunslider.umg_sunslider_C|GetSlider_67 (Variables|/Game/Alakaria_Fajar/Blueprints/UMG/umg_exterior.umg_exterior_C|Getumg_sunslider (Variables|Default|Getumg_exterior))) 1.0)
    (elif (<= _returnvalue 0.0)
      (Class|Slider|SetValue (Variables|/Game/Alakaria_Fajar/Blueprints/UMG/umg_sunslider.umg_sunslider_C|GetSlider_67 (Variables|/Game/Alakaria_Fajar/Blueprints/UMG/umg_exterior.umg_exterior_C|Getumg_sunslider (Variables|Default|Getumg_exterior))) 0.0)))
  (Class|Slider|SetValue (Variables|/Game/Alakaria_Fajar/Blueprints/UMG/umg_sunslider.umg_sunslider_C|GetSlider_67 (Variables|/Game/Alakaria_Fajar/Blueprints/UMG/umg_exterior.umg_exterior_C|Getumg_sunslider (Variables|Default|Getumg_exterior))) (+ _returnvalue (* Value 0.01))))

(event EventPlaySoundUI
  (params (Sound :type enum_soundUI%20Enum :default "NewEnumerator0"))
  (switch Utilities|FlowControl|Switch|Switchonenum_soundUI Sound
    (:NewEnumerator0
      (Audio|PlaySound2D "/Game/Alakaria_Fajar/Audio/UI/switch29.switch29" 1.0 1.0 0.12 0 0))
    (:NewEnumerator1
      (Audio|PlaySound2D "/Game/Alakaria_Fajar/Audio/UI/mouserelease1.mouserelease1" 1.0 1.0 0.12 0 0))
    (:NewEnumerator2
      (Audio|PlaySound2D 0 1.0 1.0 0.0 0 0))
    (:NewEnumerator3
      (Audio|PlaySound2D 0 1.0 1.0 0.0 0 0))))

(event EventPlayModeWalk
  ;[0.15 0.15 0.15 0.5] control mode
  (Variables|Default|SetbShowMouseCursor false)
  (Input|SetIgnoreLookInput false)
  (Input|SetInputModeGameOnly self false)
  (Pawn|Components|CharacterMovement|SetMovementMode (Variables|/Script/Engine.Character|GetCharacterMovement (Variables|Default|Getchar_akaria_walk)) "MOVE_Walking" 0))

(event EventUmgMode
  ;[0.15 0.15 0.15 0.5] control mode
  (Variables|Default|SetbShowMouseCursor true)
  (Input|SetIgnoreLookInput true)
  (Input|SetInputModeGameandUI self 0 "DoNotLock" false false)
  (Utilities|IsValid (Game|GetPlayerCharacter 0)
    (:Is%20Valid
      (Pawn|Components|CharacterMovement|SetMovementMode (Variables|/Script/Engine.Character|GetCharacterMovement (Variables|Default|Getchar_akaria_walk)) "MOVE_None" 0))))

(event EventPlayModeOrbital
  ;[0.15 0.15 0.15 0.5] control mode
  (Variables|Default|SetbShowMouseCursor true)
  (Input|SetIgnoreLookInput false)
  (Input|SetInputModeGameandUI self 0 "DoNotLock" false false))

(event EventExteriorMode
  (params (Exterior%20Mode :type enum_exterior_mode%20Enum :default "NewEnumerator0"))
  ;[0.15 0.15 0.15 0.5] switch mode
  (bind _output_get (Variables|Default|SetExterior%20Mode Exterior%20Mode))
  (switch Utilities|FlowControl|Switch|Switchonenum_exterior_mode _output_get
    (:NewEnumerator0
      (Game|Player|SetViewTargetwithBlend (Variables|Default|Getchar_akaria_walk) 1.0 "VTBlend_EaseInOut" 2.0 false)
      (CallFunction|ShowSunSlider false)
      (Utilities|FlowControl|Delay 1.0)
      (Pawn|Possess (Variables|Default|Getchar_akaria_walk))
      (Class|WidgetSwitcher|SetActiveWidgetIndex (Variables|/Game/Alakaria_Fajar/Blueprints/UMG/btn_switch_exterior_mode.btn_switch_exterior_mode_C|GetWidgetSwitcher_exteriormode (Variables|/Game/Alakaria_Fajar/Blueprints/UMG/umg_menu.umg_menu_C|Getbtn_switch_exterior_mode (Variables|/Game/Alakaria_Fajar/Blueprints/UMG/umg_exterior.umg_exterior_C|Getumg_menu (Variables|Default|Getumg_exterior)))) 1))
    (:NewEnumerator1
      (CallFunction|ShowInteract false)
      (Game|Player|SetViewTargetwithBlend (Variables|Default|Getpawn_alakaria_orbital) 1.0 "VTBlend_EaseInOut" 2.0 false)
      (CallFunction|ShowSunSlider true)
      (Utilities|FlowControl|Delay 1.0)
      (Pawn|Possess (Variables|Default|Getpawn_alakaria_orbital))
      (Class|WidgetSwitcher|SetActiveWidgetIndex (Variables|/Game/Alakaria_Fajar/Blueprints/UMG/btn_switch_exterior_mode.btn_switch_exterior_mode_C|GetWidgetSwitcher_exteriormode (Variables|/Game/Alakaria_Fajar/Blueprints/UMG/umg_menu.umg_menu_C|Getbtn_switch_exterior_mode (Variables|/Game/Alakaria_Fajar/Blueprints/UMG/umg_exterior.umg_exterior_C|Getumg_menu (Variables|Default|Getumg_exterior))))))))

(event EventShowMenu
  (params (Show :type Boolean))
  ;[0.15 0.15 0.15 0.5] menu
  (Default|ToggleMenu (Variables|Default|Getumg_exterior) Show)
  (Variables|Default|SetActiveWindow (select Show "NewEnumerator0" "NewEnumerator3"))
  (if Show
    (CallFunction|UmgMode)
    (else
      (Utilities|IsValid (Game|GetPlayerCharacter 0)
        (:Is%20Valid
          (CallFunction|PlayModeWalk))
        (:Is%20Not%20Valid
          (CallFunction|PlayModeOrbital))))))

(event EventShowGuide
  (params (Show :type Boolean))
  ;[0.15 0.15 0.15 0.5] guide
  (Default|ToggleGuide (Variables|Default|Getumg_exterior) Show)
  (Variables|Default|SetActiveWindow (select Show "NewEnumerator1" "NewEnumerator3"))
  (if Show
    (CallFunction|UmgMode)
    (else
      (Utilities|IsValid (Game|GetPlayerCharacter 0)
        (:Is%20Valid
          (CallFunction|PlayModeWalk))
        (:Is%20Not%20Valid
          (CallFunction|PlayModeOrbital))))))

(event EventShowTeleport
  (params (Show :type Boolean))
  ;[0.15 0.15 0.15 0.5] teleport
  (Default|ToggleTeleport (Variables|Default|Getumg_exterior) Show)
  (Variables|Default|SetActiveWindow (select Show "NewEnumerator2" "NewEnumerator3"))
  (if Show
    (CallFunction|UmgMode)
    (else
      (Utilities|IsValid (Game|GetPlayerCharacter 0)
        (:Is%20Valid
          (CallFunction|PlayModeWalk))
        (:Is%20Not%20Valid
          (CallFunction|PlayModeOrbital))))))

(event EventShowHouseInfo
  (params (Show :type Boolean) (House%20Type :type enum_house_type%20Enum :default "NewEnumerator0") (Toggle :type Boolean))
  (bind _umg_exterior (Variables|Default|Getumg_exterior))
  (bind _umg_house_info (Variables|/Game/Alakaria_Fajar/Blueprints/UMG/umg_exterior.umg_exterior_C|Getumg_house_info _umg_exterior))
  (bind _returnvalue (Widget|IsVisible _umg_house_info))
  (bind _returnvalue_2 (not _returnvalue))
  (bind _returnvalue_3 (select Toggle _returnvalue_2 Show))
  ;[0.15 0.15 0.15 0.5] house info
  (switch Utilities|FlowControl|Switch|Switchonenum_umg_windows (Variables|Default|GetActiveWindow)
    (:NewEnumerator3
      _)
    (:NewEnumerator4
      _))
  (if _returnvalue_3
    (CallFunction|SetHouseInfo House%20Type))
  (Default|ToggleHouseinfo (Variables|Default|Getumg_exterior) _returnvalue_3)
  (Variables|Default|SetActiveWindow (select _returnvalue_3 "NewEnumerator4" "NewEnumerator3"))
  (if _returnvalue_3
    (CallFunction|UmgMode)
    (else
      (Utilities|IsValid (Game|GetPlayerCharacter 0)
        (:Is%20Valid
          (CallFunction|PlayModeWalk))
        (:Is%20Not%20Valid
          (CallFunction|PlayModeOrbital))))))

(event Input|ActionEvents|InputActionMenu
  (params (Key :type Key%20Structure :default "None"))
  ;[0.15 0.15 0.15 0.5] menu
  (:Released
    (switch Utilities|FlowControl|Switch|Switchonenum_umg_windows (Variables|Default|GetActiveWindow)
      (:NewEnumerator3
        _)
      (:NewEnumerator0
        _))
    (CallFunction|ShowMenu (not (Widget|IsVisible (Variables|/Game/Alakaria_Fajar/Blueprints/UMG/umg_exterior.umg_exterior_C|Getumg_menu (Variables|Default|Getumg_exterior)))))))

(event Input|ActionEvents|InputActionGuide
  (params (Key :type Key%20Structure :default "None"))
  ;[0.15 0.15 0.15 0.5] guide
  (:Released
    (switch Utilities|FlowControl|Switch|Switchonenum_umg_windows (Variables|Default|GetActiveWindow)
      (:NewEnumerator3
        _)
      (:NewEnumerator1
        _))
    (CallFunction|ShowGuide (not (Widget|IsVisible (Variables|/Game/Alakaria_Fajar/Blueprints/UMG/umg_exterior.umg_exterior_C|Getumg_guide (Variables|Default|Getumg_exterior)))))))

(event Input|ActionEvents|InputActionTeleport
  (params (Key :type Key%20Structure :default "None"))
  ;[0.15 0.15 0.15 0.5] teleport
  (:Released
    (if (not (== (Game|Player|GetPlayerPawn 0) (Variables|Default|Getpawn_alakaria_orbital)))
      (switch Utilities|FlowControl|Switch|Switchonenum_umg_windows (Variables|Default|GetActiveWindow)
        (:NewEnumerator3
          _)
        (:NewEnumerator2
          _))
      (CallFunction|ShowTeleport (not (Widget|IsVisible (Variables|/Game/Alakaria_Fajar/Blueprints/UMG/umg_exterior.umg_exterior_C|Getumg_teleport (Variables|Default|Getumg_exterior))))))))

(event Input|KeyboardEvents|NumPadOne
  (params (Key :type Key%20Structure :default "None"))
  (:Released
    (Utilities|SetDLSS/DLAAMode(noAuto) "Off" false false)))

(event Input|GamepadEvents|GamepadDPadLeft
  (params (Key :type Key%20Structure :default "None"))
  ;[0.15 0.15 0.15 0.5] guide
  (:Released
    (switch Utilities|FlowControl|Switch|Switchonenum_umg_windows (Variables|Default|GetActiveWindow)
      (:NewEnumerator1
        (Default|SetActiveKeyButton (Variables|/Game/Alakaria_Fajar/Blueprints/UMG/umg_guide.umg_guide_C|Getbtn_inputkey_mkey (Variables|/Game/Alakaria_Fajar/Blueprints/UMG/umg_exterior.umg_exterior_C|Getumg_guide (Variables|Default|Getumg_exterior))))
        (CallFunction|PlaySoundUI "NewEnumerator1")))))

(event Input|GamepadEvents|GamepadDPadRight
  (params (Key :type Key%20Structure :default "None"))
  ;[0.15 0.15 0.15 0.5] guide
  (:Released
    (switch Utilities|FlowControl|Switch|Switchonenum_umg_windows (Variables|Default|GetActiveWindow)
      (:NewEnumerator1
        (Default|SetActiveKeyButton (Variables|/Game/Alakaria_Fajar/Blueprints/UMG/umg_guide.umg_guide_C|Getbtn_inputkey_gamepad (Variables|/Game/Alakaria_Fajar/Blueprints/UMG/umg_exterior.umg_exterior_C|Getumg_guide (Variables|Default|Getumg_exterior))))
        (CallFunction|PlaySoundUI "NewEnumerator1")))))

(event Input|KeyboardEvents|NumPadTwo
  (params (Key :type Key%20Structure :default "None"))
  (:Released
    (Utilities|SetDLSS/DLAAMode(noAuto) "Auto" false false)))

(event Input|KeyboardEvents|NumPadThree
  (params (Key :type Key%20Structure :default "None"))
  (:Released
    (Utilities|SetDLSS/DLAAMode(noAuto) "DLAA" true false)))

(event Input|KeyboardEvents|NumPadFour
  (params (Key :type Key%20Structure :default "None"))
  (:Released
    (Utilities|SetDLSS/DLAAMode(noAuto) "UltraQuality" false false)))

(event Input|KeyboardEvents|NumPadFive
  (params (Key :type Key%20Structure :default "None"))
  (:Released
    (Utilities|SetDLSS/DLAAMode(noAuto) "Quality" false false)))

(event Input|KeyboardEvents|NumPadSix
  (params (Key :type Key%20Structure :default "None"))
  (:Released
    (Utilities|SetDLSS/DLAAMode(noAuto) "Balanced" false false)))

(event Input|KeyboardEvents|NumPadSeven
  (params (Key :type Key%20Structure :default "None"))
  (:Released
    (Utilities|SetDLSS/DLAAMode(noAuto) "Performance" false false)))

(event Input|KeyboardEvents|NumPadEight
  (params (Key :type Key%20Structure :default "None"))
  (:Released
    (Utilities|SetDLSS/DLAAMode(noAuto) "UltraPerformance" false false)))

(fn ConstructionScript)

(fn GetExteriorMode
  (return (Variables|Default|GetExterior%20Mode)))

(fn GetIsGamepadKey
  (return (Variables|Default|GetGamepadKey)))